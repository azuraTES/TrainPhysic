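; Player controller component that detects the actor under the mouse cursor as a button.
; BeginPlay caches the owning PlayerController and its camera manager.
; Each Tick runs a complex cursor trace on a custom channel, sets IsDetected, and calls the detected event with the hit actor or the lost event on every miss.
; A camera-forward line trace helper is defined, though Tick uses the cursor trace instead.
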(event `self.ReceiveBeginPlay`
  (bind _asplayer_controller (cast `PlayerController` (`self.GetOwner`)))
  (set `self.As Player Controller` _asplayer_controller)
  (set `self.Owner` (`PlayerController.PlayerCameraManager` _asplayer_controller)))

(event `self.ReceiveTick`
  (params (DeltaSeconds :type "Float (single-precision)"))
  (bind (_hitresult _returnvalue) (`PlayerController.GetHitResultUnderCursorByChannel` (`self.As Player Controller`) "TraceTypeQuery3" true))
  (if _returnvalue
    (`self.OnDetectedButton` (`.HitActor` (`GameplayStatics.BreakHitResult` _hitresult)))
    (set `self.IsDetected` true)
    (else
      (set `self.IsDetected` false)
      (`self.OnLostButton`))))

(fn `GetVectorsForLineTrace`
  (returns (Start :type "Vector Structure") (End :type "Vector Structure"))
  (bind _owner (`self.Owner`))
  (bind _returnvalue (`Actor.K2_GetActorLocation` _owner))
  (return _returnvalue (+ _returnvalue (* (`KismetMathLibrary.GetForwardVector` (`Actor.K2_GetActorRotation` _owner)) (`self.Distance`)))))