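; Branching rail switch actor that reports one of two splines as the current rail.
; PressedButton toggles which spline the switch selects, while hover events swap the cube's material as a highlight.
; Three trigger boxes compare the overlapping actor's velocity to the switch's forward vector by dot product.
; Box and Box1 force their own branch based on that direction, while Box2 applies the switched selection for forward travel.
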(event `self.ReceiveBeginPlay`
  (`parent.ReceiveBeginPlay`)
  (bind _output_get (set `self.CurrentSpline` (`self.Spline`)))
  (set `self.CurrentSplineSwitch` _output_get))

(event `/Game/Core/Blueprint/InteractiveButton/Interfaces/BI_InteractiveButtonColorManipulation.Hover`
  (`PrimitiveComponent.SetMaterial` (`self.Cube`) 0 "/DatasmithContent/Materials/AliasMaster.AliasMaster"))

(event `/Game/Core/Blueprint/InteractiveButton/Interfaces/BI_InteractiveButtonColorManipulation.Unhover`
  (`PrimitiveComponent.SetMaterial` (`self.Cube`) 0 "/Engine/BasicShapes/BasicShapeMaterial.BasicShapeMaterial"))

(event `self.Box.OnComponentBeginOverlap`
  (params (OverlappedComponent :type "PrimitiveComponent Object Reference") (OtherActor :type "Actor Object Reference") (OtherComp :type "PrimitiveComponent Object Reference") (OtherBodyIndex :type Integer) (bFromSweep :type Boolean) (SweepResult :type "HitResult Structure (by ref)"))
  (if (< (`self.FindDOT` OtherActor) 0.0)
    (set `self.CurrentSpline` (`self.Spline1`))))

(event `self.Box1.OnComponentBeginOverlap`
  (params (OverlappedComponent :type "PrimitiveComponent Object Reference") (OtherActor :type "Actor Object Reference") (OtherComp :type "PrimitiveComponent Object Reference") (OtherBodyIndex :type Integer) (bFromSweep :type Boolean) (SweepResult :type "HitResult Structure (by ref)"))
  (if (< (`self.FindDOT` OtherActor) 0.7)
    (set `self.CurrentSpline` (`self.Spline`))))

(event `self.Box2.OnComponentBeginOverlap`
  (params (OverlappedComponent :type "PrimitiveComponent Object Reference") (OtherActor :type "Actor Object Reference") (OtherComp :type "PrimitiveComponent Object Reference") (OtherBodyIndex :type Integer) (bFromSweep :type Boolean) (SweepResult :type "HitResult Structure (by ref)"))
  (if (not (< (`self.FindDOT` OtherActor) 0.0))
    (set `self.CurrentSpline` (`self.CurrentSplineSwitch`))))

(fn `FindDOT`
  (params (Actor :type "Actor Object Reference"))
  (returns (Dot :type "Float (double-precision)"))
  (return (`KismetMathLibrary.Dot_VectorVector` (`KismetMathLibrary.Normal` (`self.GetVelocity` Actor)) (`KismetMathLibrary.Normal` (`self.GetActorForwardVector`)))))

(fn `GetCurrentRail`
  (returns (CurrentRail :type "SplineComponent Object Reference"))
  (return (`self.CurrentSpline`)))

(fn `IsRailWithBranch`
  (returns (IsRailWithBranch :type Boolean))
  (return true))

(fn `PressedButton`
  (if (`self.Switcher`)
    (set `self.Switcher` false)
    (set `self.CurrentSplineSwitch` (`self.Spline`))
    (return)
    (else
      (set `self.Switcher` true)
      (set `self.CurrentSplineSwitch` (`self.Spline1`))
      (return))))

(fn `UserConstructionScript`)