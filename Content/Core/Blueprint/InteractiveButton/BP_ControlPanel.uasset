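; Train control panel actor that populates itself with interactive buttons for operating a Locomotive.
; On BeginPlay, SpawnButtons spawns one single, one long and two switch button actors, passing each the Locomotive as OwnerTrain and its own TypeControlTrain value.
; Each button is snapped to a dedicated root component on the panel, keeping relative scale; button behavior lives in the spawned classes.
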(event `self.ReceiveBeginPlay`
  (`self.SpawnButtons`))

(event `SpawnButtons`
  (bind _returnvalue (`|SpawnActorFromClass` "/Game/Core/Blueprint/InteractiveButton/BP_InteractiveButtonSingle.BP_InteractiveButtonSingle_C" (`self.Spawn Transform`) "Undefined" "OverrideRootScale" null (`self.Locomotive`) "NewEnumerator1" null))
  (`self.K2_AttachToComponent` _returnvalue (`self.RootForSimpleButton`) "None" "SnapToTarget" "SnapToTarget" "KeepRelative" true)
  (bind _returnvalue_2 (`|SpawnActorFromClass` "/Game/Core/Blueprint/InteractiveButton/BP_InteractiveButtonLong.BP_InteractiveButtonLong_C" (`self.Spawn Transform`) "Undefined" "OverrideRootScale" null (`self.Locomotive`) "NewEnumerator2" null))
  (`self.K2_AttachToComponent` _returnvalue_2 (`self.RootForLongButton`) "None" "SnapToTarget" "SnapToTarget" "KeepRelative" true)
  (bind _returnvalue_3 (`|SpawnActorFromClass` "/Game/Core/Blueprint/InteractiveButton/BP_InteractiveButtonSwith.BP_InteractiveButtonSwith_C" (`self.Spawn Transform`) "Undefined" "OverrideRootScale" null (`self.Locomotive`) "NewEnumerator3" null))
  (`self.K2_AttachToComponent` _returnvalue_3 (`self.RootForSwithButton`) "None" "SnapToTarget" "SnapToTarget" "KeepRelative" true)
  (bind _returnvalue_4 (`|SpawnActorFromClass` "/Game/Core/Blueprint/InteractiveButton/BP_InteractiveButtonSwith.BP_InteractiveButtonSwith_C" (`self.Spawn Transform`) "Undefined" "OverrideRootScale" null (`self.Locomotive`) "NewEnumerator4" null))
  (`self.K2_AttachToComponent` _returnvalue_4 (`self.RootForSwithButton1`) "None" "SnapToTarget" "SnapToTarget" "KeepRelative" true))

(fn `UserConstructionScript`)