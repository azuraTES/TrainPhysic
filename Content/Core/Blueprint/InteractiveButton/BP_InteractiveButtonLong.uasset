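; BP_InteractiveButtonLong is an interactive button Blueprint that extends its parent's press and release events with a repeating timer for as long as it is held.
; Pressing calls the parent, then starts a looping 0.1-second timer bound to TimerEvent and stores its handle.
; Releasing calls the parent, then clears and invalidates that timer.
; TimerEvent has no logic in this Blueprint.
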(event `self.PressedEvent`
  (`parent.PressedEvent`)
  (bind _returnvalue (`KismetSystemLibrary.K2_SetTimerDelegate` (delegate `TimerEvent`) 0.1 true))
  (set `self.Timer` _returnvalue))

(event `TimerEvent`)

(event `self.ReleasedEvent`
  (`parent.ReleasedEvent`)
  (`KismetSystemLibrary.K2_ClearAndInvalidateTimerHandle` (`self.Timer`)))

(fn `UserConstructionScript`
  (`parent.UserConstructionScript`))