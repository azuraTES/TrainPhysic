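; Base Blueprint for an interactive train control button that reports presses to its owning train.
; Hover and Unhover set a pre-activation flag and swap the mesh material to show focus.
; PressedButton only fires while pre-activated, changing the material and sending its control type to OwnerTrain, and otherwise prints an error.
; ReleasedButton clears the pressed state and restores the hover material without checking hover.
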(event `/Game/Core/Blueprint/InteractiveButton/Interfaces/BI_InteractiveButtonColorManipulation.Hover`
  ;[1 1 1] Show/Hide Widget and prepare button for press
  (`PrimitiveComponent.SetMaterial` (`self.StaticMesh`) 1 "/Engine/MapTemplates/Materials/BasicAsset03.BasicAsset03")
  (set `self.PreActivation` true))

(event `/Game/Core/Blueprint/InteractiveButton/Interfaces/BI_InteractiveButtonColorManipulation.Unhover`
  ;[1 1 1] Show/Hide Widget and prepare button for press
  (`PrimitiveComponent.SetMaterial` (`self.StaticMesh`) 1 "/Engine/BasicShapes/BasicShapeMaterial.BasicShapeMaterial")
  (set `self.PreActivation` false))

(event `PressedEvent`
  ;[1 1 1] ChangeColor
  (set `self.IsPressed` true)
  (`PrimitiveComponent.SetMaterial` (`self.StaticMesh`) 1 "/Engine/MapTemplates/Materials/BasicAsset01.BasicAsset01")
  (message `/Game/Core/Blueprint/Train/Interface/BI_TrainControl.ButtonInput` (`self.OwnerTrain`) (`self.TypeControlTrain`)))

(event `ReleasedEvent`
  ;[1 1 1] ChangeColor
  (set `self.IsPressed` false)
  (`PrimitiveComponent.SetMaterial` (`self.StaticMesh`) 1 "/Engine/MapTemplates/Materials/BasicAsset03.BasicAsset03"))

(event `/Game/Core/Blueprint/InteractiveButton/Interfaces/BI_InteractiveButtonManipulation.ReleasedButton`
  (`self.ReleasedEvent`))

(event `/Game/Core/Blueprint/InteractiveButton/Interfaces/BI_InteractiveButtonManipulation.PressedButton`
  (if (`self.PreActivation`)
    (`self.PressedEvent`)
    (else
      (`KismetSystemLibrary.PrintString` "Error:: Try Press Button without overlap"))))

(fn `UserConstructionScript`)