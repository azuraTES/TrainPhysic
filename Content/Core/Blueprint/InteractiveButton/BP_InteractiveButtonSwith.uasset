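; BP_InteractiveButtonSwith is an interactive button variant that acts as a toggle switch.
; Each press runs the parent logic, flips SwithState and, if ShouldSwitherHaveTimer is set, starts a short looping timer bound to TimerEvent.
; Release runs the parent logic and clears any valid timer, so ticking is meant to last only while held.
; TimerEvent is empty here, so the repeating tick has no effect in this Blueprint.
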(event `self.PressedEvent`
  (`parent.PressedEvent`)
  (set `self.SwithState` (not (`self.SwithState`)))
  (if (`self.ShouldSwitherHaveTimer`)
    (bind _returnvalue (`KismetSystemLibrary.K2_SetTimerDelegate` (delegate `TimerEvent`) 0.1 true))
    (set `self.Timer` _returnvalue)))

(event `TimerEvent`)

(event `self.ReleasedEvent`
  (`parent.ReleasedEvent`)
  (if (`KismetSystemLibrary.K2_IsValidTimerHandle` (`self.Timer`))
    (`KismetSystemLibrary.K2_ClearAndInvalidateTimerHandle` (`self.Timer`))))

(fn `UserConstructionScript`
  (`parent.UserConstructionScript`))