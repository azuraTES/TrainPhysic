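; BP_SimpleWagonTrain is a train wagon that gets a physics-linked coupler at each of its two constraint points.
; On BeginPlay, after the parent logic, it spawns two BP_CouplerWagon actors at the transforms of PhysicsConstraint and PhysicsConstraint1.
; Each constraint then joins TrainBody to its coupler's Cube at runtime, so the couplers are separate actors attached through physics.
; The construction script only calls the parent.
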(event `self.ReceiveBeginPlay`
  (`parent.ReceiveBeginPlay`)
  ;[1 1 1] Spawn coupler
  (bind _returnvalue (`|SpawnActorFromClass` "/Game/Core/Blueprint/Train/Coupler/BP_CouplerWagon.BP_CouplerWagon_C" (`SceneComponent.K2_GetComponentToWorld` (`self.PhysicsConstraint`)) "AlwaysSpawn" "OverrideRootScale" null null))
  (`PhysicsConstraintComponent.SetConstrainedComponents` (`self.PhysicsConstraint`) (`self.TrainBody`) "None" (`/Game/Core/Blueprint/Train/Coupler/BP_CouplerWagon.Cube` _returnvalue) "None")
  (bind _returnvalue_2 (`|SpawnActorFromClass` "/Game/Core/Blueprint/Train/Coupler/BP_CouplerWagon.BP_CouplerWagon_C" (`SceneComponent.K2_GetComponentToWorld` (`self.PhysicsConstraint1`)) "AlwaysSpawn" "OverrideRootScale" null null))
  (`PhysicsConstraintComponent.SetConstrainedComponents` (`self.PhysicsConstraint1`) (`self.TrainBody`) "None" (`/Game/Core/Blueprint/Train/Coupler/BP_CouplerWagon.Cube` _returnvalue_2) "None"))

(fn `UserConstructionScript`
  (`parent.UserConstructionScript`))