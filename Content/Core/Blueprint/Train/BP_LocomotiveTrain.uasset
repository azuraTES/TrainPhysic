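; Locomotive train Blueprint that acts as the drivable engine car, delegating movement to its TraneEngine component.
; On BeginPlay it spawns a coupler wagon joined to the body by a physics constraint, plus a control panel attached at its root and linked back to the locomotive.
; ButtonInput maps throttle, brake toggle, speed limit and direction change to engine calls.
; It binds to the engine's direction-change event.
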(event `self.ReceiveBeginPlay`
  (`parent.ReceiveBeginPlay`)
  (add `/Game/Core/Blueprint/Train/Component/BP_TraneEngineComponent.OnChangeDirectionOfMovement` (`self.TraneEngine`) (`|CreateDelegate` :!event `SetNewDirectionOfMovement`))
  ;[1 1 1] Spawn coupler
  (bind _returnvalue (`|SpawnActorFromClass` "/Game/Core/Blueprint/Train/Coupler/BP_CouplerWagon.BP_CouplerWagon_C" (`SceneComponent.K2_GetComponentToWorld` (`self.PhysicsConstraint`)) "AlwaysSpawn" "OverrideRootScale" null null))
  (`PhysicsConstraintComponent.SetConstrainedComponents` (`self.PhysicsConstraint`) (`self.TrainBody`) "None" (`/Game/Core/Blueprint/Train/Coupler/BP_CouplerWagon.Cube` _returnvalue) "None")
  (bind _returnvalue_2 (`|SpawnActorFromClass` "/Game/Core/Blueprint/InteractiveButton/BP_ControlPanel.BP_ControlPanel_C" (`SceneComponent.K2_GetComponentToWorld` (`self.ControlPanelRoot`)) "AlwaysSpawn" "OverrideRootScale" null self null))
  (`self.K2_AttachToComponent` _returnvalue_2 (`self.ControlPanelRoot`) "None" "SnapToTarget" "SnapToTarget" "SnapToTarget" false))

(event `/Game/Core/Blueprint/Train/Interface/BI_TrainControl.ButtonInput`
  (params (InputID :type "/Game/Core/Blueprint/InteractiveButton/Enum/E_TypeControlTrain Enum" :default "NewEnumerator0"))
  ;[1 1 1] Input for train
  (switch `/Game/Core/Blueprint/InteractiveButton/Enum/E_TypeControlTrain` InputID
    (:`NewEnumerator1`
      (`/Game/Core/Blueprint/Train/Component/BP_TraneEngineComponent.AddSpeed` (`self.TraneEngine`)))
    (:`NewEnumerator2`
      (`self.BrakeSwither`))
    (:`NewEnumerator3`
      (`/Game/Core/Blueprint/Train/Component/BP_TraneEngineComponent.ActivateAutoSpeedControl` (`self.TraneEngine`) (`self.Max Speed`)))
    (:`NewEnumerator4`
      (`/Game/Core/Blueprint/Train/Component/BP_TraneEngineComponent.ChangeDirectionOfMovement` (`self.TraneEngine`)))))

(event `BrakeSwither`
  ;[1 1 1] BrakeSwither
  (if (`self.IsBrake`)
    (set `self.IsBrake` false)
    (`/Game/Core/Blueprint/Train/Component/BP_TraneEngineComponent.DeactivateBrake` (`self.TraneEngine`))
    (else
      (set `self.IsBrake` true)
      (`/Game/Core/Blueprint/Train/Component/BP_TraneEngineComponent.ActivateBrake` (`self.TraneEngine`)))))

(event `SetNewDirectionOfMovement`
  (params (CurrentDirectionOfMovement :type Name))
  ;[1 1 1] Set new direction
  (set `self.Current Direction Of Movement` CurrentDirectionOfMovement))

(fn `UserConstructionScript`
  (`parent.UserConstructionScript`))