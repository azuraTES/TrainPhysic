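; BP_CouplerWagon is a train wagon coupler that aims at, links to and releases from another coupler.
; An outer finder overlap starts a looping timer that turns the coupler mesh toward the other coupler's mesh.
; The constraint trigger's overlap joins both meshes at their sockets with a physics constraint, then disables itself and stops the aiming.
; PressedButton breaks the constraint, restarts aiming and re-enables the trigger.
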(event `self.CouplerFounder.OnComponentBeginOverlap`
  (params (OverlappedComponent :type "PrimitiveComponent Object Reference") (OtherActor :type "Actor Object Reference") (OtherComp :type "PrimitiveComponent Object Reference") (OtherBodyIndex :type Integer) (bFromSweep :type Boolean) (SweepResult :type "HitResult Structure (by ref)"))
  (bind _asbp_coupler_wagon (cast `/Game/Core/Blueprint/Train/Coupler/BP_CouplerWagon` OtherActor))
  (set `self.As BP Coupling Wagon` _asbp_coupler_wagon)
  (`self.StartCheckCouplingWagon`))

(event `self.CouplerFounder.OnComponentEndOverlap`
  (params (OverlappedComponent :type "PrimitiveComponent Object Reference") (OtherActor :type "Actor Object Reference") (OtherComp :type "PrimitiveComponent Object Reference") (OtherBodyIndex :type Integer))
  (`KismetSystemLibrary.K2_ClearAndInvalidateTimerHandle` (`self.TimerCheck`))
  (set `self.As BP Coupling Wagon` null))

(event `StartCheckCouplingWagon`
  (bind _returnvalue (`KismetSystemLibrary.K2_SetTimerDelegate` (delegate `RotateCouplingWagon`) 0.1 true))
  (set `self.TimerCheck` _returnvalue))

(event `RotateCouplingWagon`
  (`SceneComponent.K2_SetWorldRotation` (`self.Cube`) (`KismetMathLibrary.FindLookAtRotation` (`SceneComponent.K2_GetComponentLocation` (`self.Cube`)) (`SceneComponent.K2_GetComponentLocation` (`/Game/Core/Blueprint/Train/Coupler/BP_CouplerWagon.Cube` (`self.As BP Coupling Wagon`)))) false false))

(event `DisablePhysicsConstrain`
  (`PhysicsConstraintComponent.BreakConstraint` (`self.PhysicsConstraint`))
  (`self.StartCheckCouplingWagon`)
  (`PrimitiveComponent.SetCollisionEnabled` (`self.CouplerConstraint`) "QueryOnly"))

(event `self.CouplerConstraint.OnComponentBeginOverlap`
  (params (OverlappedComponent :type "PrimitiveComponent Object Reference") (OtherActor :type "Actor Object Reference") (OtherComp :type "PrimitiveComponent Object Reference") (OtherBodyIndex :type Integer) (bFromSweep :type Boolean) (SweepResult :type "HitResult Structure (by ref)"))
  (bind _asbp_coupler_wagon (cast `/Game/Core/Blueprint/Train/Coupler/BP_CouplerWagon` OtherActor))
  (`PhysicsConstraintComponent.SetConstrainedComponents` (`self.PhysicsConstraint`) (`self.Cube`) "CouplerSocket" (`/Game/Core/Blueprint/Train/Coupler/BP_CouplerWagon.Cube` _asbp_coupler_wagon) "CouplerSocket")
  (`PrimitiveComponent.SetCollisionEnabled` (`self.CouplerConstraint`) "NoCollision")
  (`KismetSystemLibrary.K2_ClearAndInvalidateTimerHandle` (`self.TimerCheck`)))

(fn `PressedButton`
  (`self.DisablePhysicsConstrain`)
  (`KismetSystemLibrary.PrintString` "Hello")
  (return))

(fn `UserConstructionScript`)