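; Base train wagon that rides spline rails as a physics body and derails when it loses them.
; Each tick, spring-damper forces pull both carriage sockets toward the current spline, leaving motion along it free, while a damped torque corrects roll.
; A looping timer traces down to update the spline from the rail below.
; Missing rail, mismatched switch branches, or excessive speed combined with high corrective torque disable rail following.
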(event `self.ReceiveBeginPlay`
  (set `self.Current Direction Of Movement` "ForwardCarriage")
  (set `self.CurrentSplineComponent` (`self.GetComponentByClass` (`self.CurrentRailActor`) "/Script/Engine.SplineComponent"))
  (`self.StartCheckRails`))

(event `self.ReceiveTick`
  (params (DeltaSeconds :type "Float (single-precision)"))
  (`self.CurrentSplineComponent`
    (:`then`
      (`self.ProcessCarriage` "ForwardCarriage")
      (`self.ProcessCarriage` "BackwardCarriage")
      (`self.ControlRotation`))
    (:`else`
      (`KismetSystemLibrary.PrintString` "not valid"))))

(event `DisableTrain`
  ;[1 1 1] DeactivateTrain
  (`PrimitiveComponent.PutRigidBodyToSleep` (`self.TrainBody`) "None")
  (set `self.CurrentSplineComponent` null)
  (set `self.ShouldDisableTrain` false)
  (`KismetSystemLibrary.K2_ClearAndInvalidateTimerHandle` (`self.CheckRailsTimer`)))

(event `StartCheckRails`
  (bind _returnvalue (`KismetSystemLibrary.K2_SetTimerDelegate` (delegate `CheckRails`) 0.05 true))
  (set `self.CheckRailsTimer` _returnvalue))

(event `CheckRails`
  (`self.CheckRailsFromCarriage` (`self.Current Direction Of Movement`)))

(event `CheckRailsFromCarriage`
  (params (SocketName :type Name))
  ;[1 1 1] Check simple rails
  (bind (_outhit _washit) (`self.GetHitFromSocket` SocketName))
  (if _washit
    (bind (_bblockinghit _binitialoverlap _time _distance _location _impactpoint _normal _impactnormal _physmat _hitactor) (`GameplayStatics.BreakHitResult` _outhit))
    (bind _output_get (set `self.CurrentRailActor` _hitactor))
    (bind _currentrail (message `/Game/Core/Blueprint/Train/Interface/BI_SetNewRails.GetCurrentRail` _output_get))
    (set `self.CurrentSplineComponent` _currentrail)
    ;[1 1 1] CheckSwith rails
    (bind _israilwithbranch (message `/Game/Core/Blueprint/Train/Interface/BI_SetNewRails.IsRailWithBranch` _hitactor))
    (if _israilwithbranch
      (for _array_element (`SceneComponent.GetAllSocketNames` (`self.TrainBody`))
        (if (!= _array_element (`self.Current Direction Of Movement`))
          (bind _outhit_2 (`self.GetHitFromSocket` _array_element))
          (bind (_bblockinghit_2 _binitialoverlap_2 _time_2 _distance_2 _location_2 _impactpoint_2 _normal_2 _impactnormal_2 _physmat_2 _hitactor_2) (`GameplayStatics.BreakHitResult` _outhit_2))
          (if (== _hitactor_2 (`self.CurrentRailActor`))
            (bind _currentrail_2 (message `/Game/Core/Blueprint/Train/Interface/BI_SetNewRails.GetCurrentRail` _hitactor_2))
            (if (!= _currentrail_2 (`self.CurrentSplineComponent`))
              (set `self.ShouldDisableTrain` true)))))
      (if (`self.ShouldDisableTrain`)
        (`self.DisableTrain`)))
    (else
      (`self.DisableTrain`))))

(fn `ControlRotation`
  (locals (TrainRotation :type "Rotator Structure" :default (struct)) (MaxVelocity :type "Float (double-precision)" :default 1500.0) (MaxTorgue :type "Float (double-precision)" :default 3000.0) (RotationStiffness :type "Float (double-precision)" :default 1000.0) (RotationDamping :type "Float (double-precision)" :default 10.0))
  (bind (_trainrotation_roll _trainrotation_pitch _trainrotation_yaw) (`KismetMathLibrary.BreakRotator` (`local.TrainRotation`)))
  (bind _returnvalue (`KismetMathLibrary.GetForwardVector` (`local.TrainRotation`)))
  (bind _returnvalue_2 (`KismetMathLibrary.GetRightVector` (`local.TrainRotation`)))
  (bind _returnvalue_3 (+ (* (`KismetMathLibrary.ProjectVectorOnToVector` (`PrimitiveComponent.GetPhysicsAngularVelocityInDegrees` (`self.TrainBody`) "None") _returnvalue) (* (`local.RotationDamping`) -1.0)) (* _returnvalue (* (`KismetMathLibrary.SignOfFloat` (.z _returnvalue_2)) (`KismetMathLibrary.DegAcos` (`KismetMathLibrary.Dot_VectorVector` _returnvalue_2 (`KismetMathLibrary.GetRightVector` (`KismetMathLibrary.MakeRotator` 0.0 0.0 _trainrotation_yaw)))) (`local.RotationStiffness`) -1.0))))
  (set `local.TrainRotation` (`SceneComponent.K2_GetComponentRotation` (`self.TrainBody`)))
  ;[1 1 1] Check wagon in rotation
  (`PrimitiveComponent.AddTorqueInDegrees` (`self.TrainBody`) _returnvalue_3 "None" true)
  (bind _returnvalue_4 (`PrimitiveComponent.GetPhysicsLinearVelocity` (`self.TrainBody`) "None"))
  (if (and (> (`KismetMathLibrary.VSize` _returnvalue_4) (`local.MaxVelocity`)) (> (`KismetMathLibrary.VSize` _returnvalue_3) (`local.MaxTorgue`)))
    ;[1 1 1] Disable wagon
    (`self.DisableTrain`)))

(fn `GetHitFromSocket`
  (params (SocketName :type Name))
  (returns (OutHit :type "HitResult Structure") (WasHit :type Boolean))
  (locals (`Object Types` :type "Array of EObjectTypeQuery Enum"))
  (bind (_outhit _returnvalue) (`KismetSystemLibrary.LineTraceSingle` (`SceneComponent.GetSocketLocation` (`self.TrainBody`) SocketName) (+ (`SceneComponent.GetSocketLocation` (`self.TrainBody`) SocketName) (* (* (`KismetMathLibrary.GetUpVector` (`SceneComponent.GetSocketRotation` (`self.TrainBody`) SocketName)) -1.0) 1000.0)) "TraceTypeQuery4" true))
  (return _outhit _returnvalue))

(fn `ProcessCarriage`
  (params (CarriageSocket :type Name))
  (locals (CurrentLocation :type "Vector Structure" :default (0.0 0.0 0.0)) (ProjectedToSpline :type "Transform Structure") (ForceCorrectionOffset :type "Vector Structure" :default (0.0 0.0 0.0)) (Stiffness :type "Float (double-precision)" :default 30000.0) (Damping :type "Float (double-precision)" :default 2000.0))
  (bind (_projectedtospline_location _projectedtospline_rotation) (`KismetMathLibrary.BreakTransform` (`local.ProjectedToSpline`)))
  (bind _projectedtospline_location_2 (`KismetMathLibrary.BreakTransform` (`local.ProjectedToSpline`)))
  ;[1 1 1] Prepair
  (set `local.CurrentLocation` (`SceneComponent.GetSocketLocation` (`self.TrainBody`) (`local.CarriageSocket`)))
  (set `local.ProjectedToSpline` (`SplineComponent.FindTransformClosestToWorldLocation` (`self.CurrentSplineComponent`) (`local.CurrentLocation`) "World" false))
  (set `local.ForceCorrectionOffset` (0.0 0.0 -20.0))
  ;[1 1 1] apply handle forces
  (bind _returnvalue (`PrimitiveComponent.GetPhysicsLinearVelocityAtPoint` (`self.TrainBody`) (`local.CurrentLocation`) (`local.CarriageSocket`)))
  (`PrimitiveComponent.AddForceAtLocation` (`self.TrainBody`) (`KismetMathLibrary.ProjectVectorOnToPlane` (+ (* _returnvalue (* -1.0 (`local.Damping`))) (* (- _projectedtospline_location_2 (+ (`local.CurrentLocation`) (`local.ForceCorrectionOffset`))) (`local.Stiffness`))) (`KismetMathLibrary.GetForwardVector` _projectedtospline_rotation)) (`local.CurrentLocation`) "None"))

(fn `UserConstructionScript`)