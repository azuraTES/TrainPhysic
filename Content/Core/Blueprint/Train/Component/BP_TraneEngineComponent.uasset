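; Train engine component that drives its owner's root static mesh with physics impulses along the forward or backward carriage socket.
; Each tick it applies an impulse scaled by the current throttle; reversing switches the socket and notifies listeners.
; An optional max-speed mode nudges linear damping or throttle toward the target speed.
; Braking zeroes throttle and uses a looping timer to interpolate linear damping until nearly stopped.
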(event `self.ReceiveBeginPlay`
  ;[1 1 1] InitParam
  (bind _output_get (set `self.Owner` (`self.GetOwner`)))
  (bind _asstatic_mesh_component (cast `StaticMeshComponent` (`Actor.RootComponent` _output_get)))
  (set `self.As Static Mesh Component` _asstatic_mesh_component)
  (set `self.DirectionOfMovement` (`self.ForwardCarriageSocketName`)))

(event `AddSpeed`
  (set `self.CurrentThrottle` (+ (`self.CurrentThrottle`) (`self.ThrottleCoef`))))

(event `RemoveSpeed`
  (set `self.CurrentThrottle` (- (`self.CurrentThrottle`) (`self.ThrottleCoef`))))

(event `self.ReceiveTick`
  (params (DeltaSeconds :type "Float (single-precision)"))
  (`self.SpeedControl`)
  (`self.AddImpulsFromEngine`))

(event `AddImpulsFromEngine`
  (if (!= (`self.CurrentThrottle`) 0.0)
    (`PrimitiveComponent.AddImpulse` (`self.As Static Mesh Component`) (`self.CalculateImpulse`) (`self.DirectionOfMovement`) false)))

(event `ChangeDirectionOfMovement`
  (if (== (`self.DirectionOfMovement`) (`self.ForwardCarriageSocketName`))
    (set `self.DirectionOfMovement` (`self.BackwardCarriageSocketName`))
    (else
      (set `self.DirectionOfMovement` (`self.ForwardCarriageSocketName`))))
  (`self.OnChangeDirectionOfMovement` (`self.DirectionOfMovement`)))

(event `BrakeStart`
  (set `self.CurrentThrottle` 0.0))

(event `ActivateAutoSpeedControl`
  (params (MaxSpeed :type "Float (double-precision)"))
  (set `self.Max Speed` MaxSpeed))

(event `DeactivateAutoSpeedControl`
  (set `self.Max Speed` 0.0))

(event `SpeedControl`
  (bind _max_speed (`self.Max Speed`))
  (bind _as_static_mesh_component (`self.As Static Mesh Component`))
  (bind _as_static_mesh_component_2 (`self.As Static Mesh Component`))
  (bind _returnvalue (`KismetMathLibrary.VSize` (`Actor.GetVelocity` (`self.Owner`))))
  (if (!= (`self.Max Speed`) 0.0)
    (if (`KismetMathLibrary.NearlyEqual_FloatFloat` _returnvalue _max_speed 0.5)
      _
      (elif (> _returnvalue _max_speed)
        (`PrimitiveComponent.SetLinearDamping` _as_static_mesh_component (+ (`PrimitiveComponent.GetLinearDamping` _as_static_mesh_component) 0.1))
        (elif (!= (`PrimitiveComponent.GetLinearDamping` (`self.As Static Mesh Component`)) 0.1)
          (`PrimitiveComponent.SetLinearDamping` _as_static_mesh_component_2 (- (`PrimitiveComponent.GetLinearDamping` _as_static_mesh_component_2) 0.1))
          (else
            (`self.AddSpeed`)))))))

(event `ActivateBrake`
  (set `self.CurrentThrottle` 0.0)
  (bind _returnvalue (`KismetSystemLibrary.K2_SetTimerDelegate` (delegate `InterpolateLinerDamping`) 0.2 true))
  (set `self.BrakeTimer` _returnvalue))

(event `InterpolateLinerDamping`
  (if (>= (`KismetMathLibrary.VSize` (`Actor.GetVelocity` (`self.GetOwner`))) 0.3)
    (`PrimitiveComponent.SetLinearDamping` (`self.As Static Mesh Component`) (`KismetMathLibrary.FInterpTo` (`PrimitiveComponent.GetLinearDamping` (`self.As Static Mesh Component`)) (`self.LinerDampingWithBrake`) 0.1 8.0))
    (else
      (`KismetSystemLibrary.K2_ClearAndInvalidateTimerHandle` (`self.BrakeTimer`)))))

(event `DeactivateBrake`
  (`PrimitiveComponent.SetLinearDamping` (`self.As Static Mesh Component`) (`self.LinerDampingWithoutBrake`))
  (if (`KismetSystemLibrary.K2_IsValidTimerHandle` (`self.BrakeTimer`))
    (`KismetSystemLibrary.K2_ClearAndInvalidateTimerHandle` (`self.BrakeTimer`))))

(fn `CalculateImpulse`
  (returns (ImpulsVector :type "Vector Structure"))
  (return (* (`KismetMathLibrary.GetForwardVector` (`SceneComponent.GetSocketRotation` (`self.As Static Mesh Component`) (`self.DirectionOfMovement`))) (`self.CurrentThrottle`))))

(fn `CalculateImpulseForAutoControl`
  (returns (MoreMaxSpeed :type Boolean))
  (return false))